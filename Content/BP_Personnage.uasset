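; Player character Blueprint that handles movement, camera look, jumping and spawning a projectile-named actor through Enhanced Input actions.
; Movement follows the actor's forward and right vectors, while look inputs feed controller pitch and yaw.
; The IA_LancerCubeEau action, despite its water-cube name, spawns BP_BoulleFeu at a rotated offset from the character with zero rotation, then prints a debug message.
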(event Input|EnhancedActionEvents|EnhancedInputActionIA_BougerAvantArriere
  (params (ActionValue :type Float%20%28double-precision%29) (ElapsedSeconds :type Float%20%28double-precision%29) (TriggeredSeconds :type Float%20%28double-precision%29) (InputAction :type Input%20Action%20Object%20Reference :default "/Game/Inputs/IA_BougerAvantArriere.IA_BougerAvantArriere"))
  ;[1 1 1] Bouger avant / arriére
  (Pawn|Input|AddMovementInput (Math|Vector|GetForwardVector (Transformation|GetActorRotation)) ActionValue false))

(event Input|EnhancedActionEvents|EnhancedInputActionIA_BougerGaucheDroite
  (params (ActionValue :type Float%20%28double-precision%29) (ElapsedSeconds :type Float%20%28double-precision%29) (TriggeredSeconds :type Float%20%28double-precision%29) (InputAction :type Input%20Action%20Object%20Reference :default "/Game/Inputs/IA_BougerGaucheDroite.IA_BougerGaucheDroite"))
  ;[1 1 1] Bouger gauche / droite
  (Pawn|Input|AddMovementInput (Math|Vector|GetRightVector (Transformation|GetActorRotation)) ActionValue false))

(event Input|EnhancedActionEvents|EnhancedInputActionIA_Sauter
  (params (ActionValue :type Boolean) (ElapsedSeconds :type Float%20%28double-precision%29) (TriggeredSeconds :type Float%20%28double-precision%29) (InputAction :type Input%20Action%20Object%20Reference :default "/Game/Inputs/IA_Sauter.IA_Sauter"))
  ;[1 1 1] Sauter
  (:Triggered
    (Character|Jump))
  (:Completed
    (Character|StopJumping)))

(event Input|EnhancedActionEvents|EnhancedInputActionIA_RegarderHautBas
  (params (ActionValue :type Float%20%28double-precision%29) (ElapsedSeconds :type Float%20%28double-precision%29) (TriggeredSeconds :type Float%20%28double-precision%29) (InputAction :type Input%20Action%20Object%20Reference :default "/Game/Inputs/IA_RegarderHautBas.IA_RegarderHautBas"))
  ;[1 1 1] Regarder  haut / bas
  (Pawn|Input|AddControllerPitchInput ActionValue))

(event Input|EnhancedActionEvents|EnhancedInputActionIA_RegarderGaucheDroite
  (params (ActionValue :type Float%20%28double-precision%29) (ElapsedSeconds :type Float%20%28double-precision%29) (TriggeredSeconds :type Float%20%28double-precision%29) (InputAction :type Input%20Action%20Object%20Reference :default "/Game/Inputs/IA_RegarderGaucheDroite.IA_RegarderGaucheDroite"))
  ;[1 1 1] Regarder gauche / droite
  (Pawn|Input|AddControllerYawInput ActionValue))

(event Input|EnhancedActionEvents|EnhancedInputActionIA_LancerCubeEau
  (params (ActionValue :type Boolean) (ElapsedSeconds :type Float%20%28double-precision%29) (TriggeredSeconds :type Float%20%28double-precision%29) (InputAction :type Input%20Action%20Object%20Reference :default "/Game/Inputs/IA_LancerCubeEau.IA_LancerCubeEau"))
  ;[1 1 1] Spawn du cube d'eau
  (Game|SpawnActorfromClass "/Game/BP_BoulleFeu.BP_BoulleFeu_C" (Math|Transform|MakeTransform (+ (Transformation|GetActorLocation) (Math|Vector|RotateVector (Variables|Default|GetV_Offset) (Transformation|GetActorRotation)))) "Undefined" "MultiplyWithRoot" 0 0)
  (Development|PrintString "Une sphère a été créée"))

(fn ConstructionScript)